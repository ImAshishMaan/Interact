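; Inspection actor that shows a given item mesh in a close-up view with a name and description widget while the character's input is disabled.
; Setter events adjust the mesh's height, rotation and scale.
; Left-drag rotates the mesh, the wheel zooms by changing a SceneCapture2D's clamped FOV, and right-click resets both.
; Interact restores character input, removes the widget and destroys the actor.
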(event `/Game/Bluprints/InspectItem/BI_Inspect.Inspect`
  (params (Character :type "/Game/Character/BP_MegaCharacter Object Reference") (Item :type "StaticMesh Object Reference") (`Item Name` :type Text) (`Item Description` :type Text))
  (set `self.Character` Character)
  (`StaticMeshComponent.SetStaticMesh` (`self.Item`) Item)
  (bind _returnvalue (`|CreateWidget` "/Game/Bluprints/InspectItem/WBP_Inspect.WBP_Inspect_C" (`GameplayStatics.GetPlayerController` 0) `Item Name` `Item Description`))
  (bind _output_get (set `self.InspectWIdgetRef` _returnvalue))
  (`UserWidget.AddToViewport` _output_get 0)
  (`self.DisableInput` (`self.Character`) (`GameplayStatics.GetPlayerController` 0)))

(event `EnhancedInput|/Game/Inputs/Actions/IA_Interact`
  (params (ActionValue :type Boolean) (ElapsedSeconds :type "Float (double-precision)") (TriggeredSeconds :type "Float (double-precision)") (InputAction :type "InputAction Object Reference" :default "/Game/Inputs/Actions/IA_Interact.IA_Interact"))
  (:`Triggered`
    (`self.EnableInput` (`self.Character`) (`GameplayStatics.GetPlayerController` 0))
    (bind _inspectwidgetref (`self.InspectWIdgetRef`)
      (:`then`
        (`Widget.RemoveFromParent` _inspectwidgetref)
        (set `self.InspectWIdgetRef` null)
        (`self.K2_DestroyActor`))
      (:`else`))))

(event `Set Inspect Item Location`
  (params (`Item Location` :type "Vector Structure"))
  (bind _item (`self.Item`))
  (bind _returnvalue (`SceneComponent.K2_GetComponentToWorld` _item))
  (`SceneComponent.K2_SetWorldTransform` _item (`KismetMathLibrary.MakeTransform` (`KismetMathLibrary.MakeVector` (.x (.location _returnvalue)) (.y (.location _returnvalue)) `Item Location_Z`) (.rotation _returnvalue) (.scale _returnvalue)) false false))

(event `Set Inspect Rotation`
  (params (`Item Rotation` :type "Rotator Structure"))
  (bind _item (`self.Item`))
  (bind (_returnvalue_location _returnvalue_rotation _returnvalue_scale) (`KismetMathLibrary.BreakTransform` (`SceneComponent.K2_GetComponentToWorld` _item)))
  ;[1 1 1] Set inspection rotation
  (bind _output_get (set `self.Initial Rotation` `Item Rotation`))
  (`SceneComponent.K2_SetWorldTransform` _item (`KismetMathLibrary.MakeTransform` _returnvalue_location _output_get _returnvalue_scale) false false))

(event `Set Inspect Scale`
  (params (`Inspection Scale` :type "Vector Structure"))
  ;[1 1 1] Set Inspection scale
  (`SceneComponent.SetWorldScale3D` (`self.Item`) `Inspection Scale`))

(event `Key|LeftMouseButton`
  (params (Key :type "Key Structure"))
  ;[1 1 1] Only allow to rotate when we hole left click
  (:`Pressed`
    (set `self.Rotate?` true))
  (:`Released`
    (set `self.Rotate?` false)))

(event `Key|RightMouseButton`
  (params (Key :type "Key Structure"))
  (:`Pressed`
    (`SceneComponent.K2_SetWorldRotation` (`self.Item`) (`self.Initial Rotation`) false false)
    (set `SceneCaptureComponent2D.FOVAngle` 50.0 (`self.SceneCaptureComponent2D`))))

(event `InputAxisKey|MouseX`
  (params (AxisValue :type "Float (single-precision)"))
  (if (`self.Rotate?`)
    (`SceneComponent.K2_SetWorldRotation` (`self.Item`) (`KismetMathLibrary.ComposeRotators` (`SceneComponent.K2_GetComponentRotation` (`self.Item`)) (`KismetMathLibrary.MakeRotator` 0.0 0.0 (* AxisValue -3.0))) false false)))

(event `InputAxisKey|MouseY`
  (params (AxisValue :type "Float (single-precision)"))
  (if (`self.Rotate?`)
    (`SceneComponent.K2_SetWorldRotation` (`self.Item`) (`KismetMathLibrary.ComposeRotators` (`SceneComponent.K2_GetComponentRotation` (`self.Item`)) (`KismetMathLibrary.MakeRotator` 0.0 (* AxisValue -3.0))) false false)))

(event `Key|MouseScrollUp`
  (params (Key :type "Key Structure"))
  (bind _scenecapturecomponent2d (`self.SceneCaptureComponent2D`))
  (:`Pressed`
    (set `SceneCaptureComponent2D.FOVAngle` (`KismetMathLibrary.FClamp` (- (`SceneCaptureComponent2D.FOVAngle` _scenecapturecomponent2d) 1.0) 30.0 80.0) _scenecapturecomponent2d)))

(event `Key|MouseScrollDown`
  (params (Key :type "Key Structure"))
  (bind _scenecapturecomponent2d (`self.SceneCaptureComponent2D`))
  (:`Pressed`
    (set `SceneCaptureComponent2D.FOVAngle` (`KismetMathLibrary.FClamp` (+ (`SceneCaptureComponent2D.FOVAngle` _scenecapturecomponent2d) 1.0) 30.0 80.0) _scenecapturecomponent2d)))

(fn `UserConstructionScript`)